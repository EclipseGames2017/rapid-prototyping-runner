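; Player character for a sprite-based endless runner, which creates the HUD and auto-runs along +X.
; Tick also turns the controller to face movement, accumulates DistanceTraveled from the never-updated start position, and raises walk speed past a distance threshold.
; Touch triggers jumps and starts once-per-press swipe detection, which only prints Left or Right.
; Stumble blinks the sprite and removes a life, disabling movement at zero, while AddTimeCrystal counts crystals.
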(event `self.ReceiveBeginPlay`
  (`|ExecutionSequence`
    (:`then_0`
      (bind _returnvalue (`|CreateWidget` "/Game/Blueprints/EndlessRunnerHUD.EndlessRunnerHUD_C"))
      (`UserWidget.AddToViewport` _returnvalue 0))
    (:`then_1`
      ;[1 1 1] Gets Distance Traveled
      (bind _output_get (set `self.LastPosition` (`self.K2_GetActorLocation`))))))

(event `self.ReceiveTick`
  (params (DeltaSeconds :type "Float (single-precision)"))
  (bind (_locationx _locationy) (`PlayerController.GetInputTouchState` (`GameplayStatics.GetPlayerController` 0) "Touch1"))
  (bind _returnvalue (`KismetMathLibrary.MakeVector2D` _locationx _locationy))
  (bind (_x _y) (`KismetMathLibrary.BreakVector2D` (- (`self.TouchStart2DVector`) (`self.TouchEnd2DVector`))))
  ;[1 1 1] Constant Running
  (`|ExecutionSequence`
    (:`then_0`
      (`self.AddMovementInput` (1.0 0.0 0.0)))
    (:`then_1`
      ;[1 1 1] Runs the update animation event
      (`self.UpdateAnimation`)
      (`/Engine/EditorBlueprintResources/StandardMacros.CompareFloat` (.x (`MovementComponent.Velocity` (`self.GetMovementComponent`)))
        (:`>`
          (`Controller.SetControlRotation` (`self.GetController`) (`KismetMathLibrary.MakeRotator` 0.0) :!label _label))
        (:`==`
          (if (`self.IsMovingRight`)
            (goto _label)
            (else
              (`Controller.SetControlRotation` (`self.GetController`) (`KismetMathLibrary.MakeRotator` 0.0 0.0 180.0) :!label _label_2))))
        (:`<`
          (goto _label_2))))
    (:`then_2`
      ;[1 1 1] Gets Distance Traveled
      (set `self.DistanceTraveled` (`KismetMathLibrary.FTrunc` (+ (/ (`KismetMathLibrary.VSize` (- (`self.K2_GetActorLocation`) (`self.LastPosition`))) 1000.0) (`KismetMathLibrary.Conv_IntToDouble` (`self.DistanceTraveled`)))))
      (set `self.LastPosition` (stale `self.ReceiveBeginPlay` _output_get)))
    (:`then_3`
      ;[1 1 1] Allows player to swipe left adn right.
      (if (`self.IsPressed`)
        (if (> (`KismetMathLibrary.VSize2D` (- (`self.TouchStart2DVector`) _returnvalue)) 5.0)
          (`/Engine/EditorBlueprintResources/StandardMacros.DoOnce` false :!label _label_3
            (:`Completed`
              (set `self.TouchEnd2DVector` _returnvalue)
              (if (> (`KismetMathLibrary.Abs` _x) (`KismetMathLibrary.Abs` _y))
                (if (> _x 0.0)
                  (`KismetSystemLibrary.PrintString` "Left")
                  (else
                    (`KismetSystemLibrary.PrintString` "Right")))))))))
    (:`then_4`
      ;[1 1 1] Increases speed.
      (if (>= (`self.DistanceTraveled`) 100)
        (if (>= (`CharacterMovementComponent.MaxWalkSpeed` (`self.CharacterMovement`)) 600.0)
          (set `CharacterMovementComponent.MaxWalkSpeed` 700.0 (`self.CharacterMovement`)))))))

(event `UpdateAnimation`
  ;[1 1 1] Changes to Running Animation
  ;;[1 1 1] Will removed as we dont need idle anima anymore
)

(event `InputTouch`
  (params (Location :type "Vector Structure") (FingerIndex :type "ETouchIndex Enum"))
  (bind (_locationx _locationy) (`PlayerController.GetInputTouchState` (`GameplayStatics.GetPlayerController` 0) "Touch1"))
  ;[1 1 1] Can Jump
  (:`Pressed`
    (`|ExecutionSequence`
      (:`then_0`
        (`self.Jump`))
      (:`then_1`
        ;[1 1 1] Allows player to swipe left adn right.
        (set `self.IsPressed` true)
        (set `self.TouchStart2DVector` (`KismetMathLibrary.MakeVector2D` _locationx _locationy)))))
  (:`Released`
    (`|ExecutionSequence`
      (:`then_0`
        (`self.StopJumping`))
      (:`then_1`
        (set `self.IsPressed` false)
        (goto _label_3 :!via `Reset`)))))

(event `Stumble`
  ;[1 1 1] Handles the stumble and Death
  (`|ExecutionSequence`
    (:`then_0`
      (`SceneComponent.SetVisibility` (`self.Sprite`) false false)
      (`KismetSystemLibrary.Delay` 0.2)
      (`SceneComponent.SetVisibility` (`self.Sprite`) true false)
      (`KismetSystemLibrary.Delay` 0.2)
      (`SceneComponent.SetVisibility` (`self.Sprite`) false false)
      (`KismetSystemLibrary.Delay` 0.2)
      (`SceneComponent.SetVisibility` (`self.Sprite`) true false))
    (:`then_1`
      (bind _output_get (set `self.Lives` (- (`self.Lives`) 1)))
      (if (== _output_get 0)
        (`CharacterMovementComponent.DisableMovement` (`self.CharacterMovement`))))))

(fn `AddTimeCrystal`
  (set `self.TotalTimeCrystals` (+ (`self.TotalTimeCrystals`) 1)))

(fn `UserConstructionScript`)
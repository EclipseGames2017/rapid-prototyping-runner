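; BP_TrackWall is a track section with a wall obstacle that makes the character stumble on impact.
; Resize calls the parent implementation, then moves WallRoot along X to half the section's length.
; When the Wall component hits a BP_Character, it calls Stumble and briefly disables the whole actor's collision before restoring it after a short delay.
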(event `/Game/Blueprints/TrackSections/BP_TrackBase.Resize`
  (params (Length :type Integer))
  (`parent.Resize` Length)
  (`SceneComponent.K2_SetRelativeLocation` (`self.WallRoot`) (`KismetMathLibrary.MakeVector` (`KismetMathLibrary.Conv_IntToDouble` (/ Length 2))) false false))

(event `self.Wall.OnComponentHit`
  (params (HitComponent :type "PrimitiveComponent Object Reference") (OtherActor :type "Actor Object Reference") (OtherComp :type "PrimitiveComponent Object Reference") (NormalImpulse :type "Vector Structure") (Hit :type "HitResult Structure (by ref)"))
  (bind _asbp_character (cast `/Game/Blueprints/BP_Character` OtherActor))
  (`/Game/Blueprints/BP_Character.Stumble` _asbp_character)
  (`self.SetActorEnableCollision` false)
  (`KismetSystemLibrary.Delay` 0.05)
  (`self.SetActorEnableCollision` true))

(fn `Init`)

(fn `UserConstructionScript`)
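; BP_TrackFloor is a floor piece for a track section that can be stretched to a given length.
; Its Resize event sets FloorRoot's world X scale to Length divided by 100, keeping Y and Z at one.
; The construction script calls SpawnTimeCrystal, which currently does nothing.
; Disconnected nodes there show unused spawning of time crystal actors or sprite instances and a random point within the TimeCrystalSpawn box.
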(event `self.ReceiveTick`
  (params (DeltaSeconds :type "Float (single-precision)")))

(event `self.Resize`
  (params (Length :type Integer))
  (`SceneComponent.SetWorldScale3D` (`self.Floor Root`) (`KismetMathLibrary.MakeVector` (/ (`KismetMathLibrary.Conv_IntToDouble` Length) 100.0) 1.0 1.0)))

(fn `SpawnTimeCrystal`)

(fn `UserConstructionScript`
  (`self.SpawnTimeCrystal`))
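; BP_ImpassableWall is a track section Blueprint for an impassable wall, derived from a parent that supplies its base construction.
; Its construction script runs the parent's, then resets WallRoot and Wall to unit relative scale, so the wall is only moved up, not scaled.
; The event graph holds only disabled stub events, and a leftover JumpHeight conversion is unused.
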(fn `UserConstructionScript`
  (bind _returnvalue (`KismetMathLibrary.MakeVector` 1.0 1.0 1.0))
  (`parent.UserConstructionScript`)
  ;[1 1 1] Only moving the wall up and not scaling it
  (`SceneComponent.SetRelativeScale3D` (`self.WallRoot`) _returnvalue)
  (`SceneComponent.SetRelativeScale3D` (`self.Wall`) _returnvalue))
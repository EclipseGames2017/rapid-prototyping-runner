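; BP_TrackGenerator lays out a straight track by spawning a row of BP_TrackFloor actors along world X.
; Initialize loops a fixed number of times, spacing each floor by TrackLength times 100 from the world origin and passing TrackLength to its EventResize.
; Both the construction script and BeginPlay call Initialize, with no cleanup of previously spawned floors.
; Reset and Tick are empty stubs.
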(event `self.ReceiveBeginPlay`
  (`self.Initialize`))

(fn `Initialize`
  (bind _tracklength (`self.TrackLength`))
  (bind _output_get (set `self.LastPosition` 0.0))
  (for _ (range 6)
    (bind _returnvalue (+ _output_get (* 100 (`KismetMathLibrary.Conv_IntToDouble` _tracklength))))
    (bind _returnvalue_2 (`|SpawnActorFromClass` "/Game/Blueprints/BP_TrackFloor.BP_TrackFloor_C" (`KismetMathLibrary.MakeTransform` (`KismetMathLibrary.MakeVector` _returnvalue)) "Undefined" "OverrideRootScale" null null))
    (`/Game/Blueprints/BP_TrackFloor.Event Resize` _returnvalue_2 _tracklength)
    (set `self.LastPosition` _returnvalue)))

(fn `Reset`)

(fn `Tick`)

(fn `UserConstructionScript`
  (`self.Initialize`))
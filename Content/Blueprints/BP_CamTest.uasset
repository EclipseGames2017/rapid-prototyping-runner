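; BP_CamTest is a test Blueprint that sorts components for scene captures A and B by visibility tag.
; UpdateCameras, run on construction and BeginPlay, loops over "Renderable" actors, adding each one's A-tagged components to a set.
; The B set instead gathers tagged components from this actor itself.
; CaptureA's ShowOnlyActors is set empty: the A set's array conversion goes unused, and the B set is never applied.
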(event `self.ReceiveBeginPlay`
  (`self.UpdateCameras`))

(event `UpdateCameras`
  (`|ExecutionSequence`
    (:`then_0`
      (bind _outactors (`GameplayStatics.GetAllActorsWithTag` "Renderable"))
      (bind _output_get (set `self.Renderable` _outactors))
      (for _array_element _output_get
        (`BlueprintSetLibrary.Set_AddItems` (`self.CaptureARenderable`) (`self.GetComponentsByTag` _array_element "/Script/Engine.ActorComponent" (`self.CaptureAVisibleTag`)))
        (`BlueprintSetLibrary.Set_AddItems` (`self.CaptureBRenderable`) (`self.GetComponentsByTag` "/Script/Engine.ActorComponent" (`self.CaptureBVisibleTag`)))))
    (:`then_1`
      (`BlueprintSetLibrary.Set_ToArray` (`self.CaptureARenderable`))
      (set `SceneCaptureComponent.ShowOnlyActors` _ (`self.CaptureA`)))))

(fn `UserConstructionScript`
  (`self.UpdateCameras`))
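; BP_LevelSection is a level section actor with a floor that can be placed along the X axis and resized to a given length.
; SetPosAndLength moves the actor to the given X, zeroing Y and Z, and scales FloorParent along X.
; It also sets tiling and offset on the Plane's dynamic material from length and world X.
; The construction script creates that material and applies SetPosAndLength when TestScaling is enabled.
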(fn `SetPosAndLength`
  (params (Length :type "Float (double-precision)") (`Position X` :type "Float (double-precision)"))
  (set `self.Length` Length)
  (`self.K2_SetActorLocation` (`KismetMathLibrary.MakeVector` `Position X`))
  (`MaterialInstanceDynamic.SetScalarParameterValue` (`self.Material`) "U" (/ (`self.Length`) 100.0))
  (`MaterialInstanceDynamic.SetScalarParameterValue` (`self.Material`) "Offset U" (/ (.x (`self.K2_GetActorLocation`)) 100.0))
  (`SceneComponent.SetWorldScale3D` (`self.FloorParent`) (`KismetMathLibrary.MakeVector` (/ (`self.Length`) 100.0) 1.0 1.0))
  (return))

(fn `UserConstructionScript`
  (bind _plane (`self.Plane`))
  (bind _returnvalue (`PrimitiveComponent.CreateDynamicMaterialInstance` _plane 0 (`PrimitiveComponent.GetMaterial` _plane 0)))
  (set `self.Material` _returnvalue)
  (if (`self.TestScaling`)
    (`self.SetPosAndLength` (`self.Length`) (.x (`self.K2_GetActorLocation`)))))